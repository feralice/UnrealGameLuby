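; Melee enemy that chases pawns spotted by PawnSensing via AIMoveTo and shows its health on a widget bar.
; Box overlap with the player plays a slash montage and applies damage, gated by a DoOnce that resets one second after overlap ends.
; AnyDamage plays hit sounds and lowers health; death ragdolls the mesh, removes the capsule, heals the seen player if below full, then destroys the actor and increments a kill counter.
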(event `self.ReceiveAnyDamage`
  (params (Damage :type "Float (single-precision)") (DamageType :type "DamageType Object Reference") (InstigatedBy :type "Controller Object Reference") (DamageCauser :type "Actor Object Reference"))
  (bind _capsulecomponent (`self.CapsuleComponent`))
  ;[1 1 1] Verifica se inimigo morrreu e seta variavel boleana
  (`|ExecutionSequence`
    (:`then_0`
      ;;[1 1 1] som emitido pelo inimigo ao receber tiro
      (`GameplayStatics.PlaySoundAtLocation` "/Game/Caracter/Sons/bolaHit.bolaHit" (`self.K2_GetActorLocation`) (struct) 0.5 1.0 0.0 null null null null))
    (:`then_1`
      (set `self.HealthInim` (- (`self.HealthInim`) Damage))
      (if (<= (`self.HealthInim`) 0.0)
        (`|ExecutionSequence`
          (:`then_0`
            (set `self.estaMortoInim` true)
            (`GameplayStatics.PlaySoundAtLocation` "/Game/Caracter/Sons/deathRat.deathRat" (`self.K2_GetActorLocation`) (struct) 0.5 1.0 0.0 null null null null)
            (`PrimitiveComponent.SetSimulatePhysics` (`self.Mesh`) true)
            (`PrimitiveComponent.SetCollisionProfileName` (`self.Mesh`) "Ragdoll" true)
            (`PrimitiveComponent.SetCollisionResponseToChannel` (`self.Mesh`) "ECC_Pawn" "ECR_Block")
            (`KismetSystemLibrary.Delay` 0.5)
            (`/Engine/EditorBlueprintResources/StandardMacros.IsValid` _capsulecomponent
              (:`Is Valid`
                (`ActorComponent.K2_DestroyComponent` _capsulecomponent)
                (`KismetSystemLibrary.Delay` 2.0)
                (bind _asbp_third_person_character (cast `/Game/Caracter/Blueprints/BP_ThirdPersonCharacter` (stale `self.PawnSensing.OnSeePawn` Pawn)))
                ;;[1 1 1] Player ganha 10 de vida se matar inimigo
                (if (< (`/Game/Caracter/Blueprints/BP_ThirdPersonCharacter.Health` _asbp_third_person_character) 1.0)
                  (set `/Game/Caracter/Blueprints/BP_ThirdPersonCharacter.Health` (+ (`/Game/Caracter/Blueprints/BP_ThirdPersonCharacter.Health` _asbp_third_person_character) 0.1) _asbp_third_person_character)
                  (`GameplayStatics.PlaySoundAtLocation` "/Game/StarterContent/Audio/Explosion01.Explosion01" (`self.K2_GetActorLocation`) (struct) 0.5 1.0 0.0 null null null null)
                  (`KismetSystemLibrary.Delay` 0.6))
                (`self.K2_DestroyActor`)
                (set `self.NumMortoInimCorpo` (+ (`self.NumMortoInimCorpo`) 1))))))))))

(event `self.ReceiveTick`
  (params (DeltaSeconds :type "Float (single-precision)"))
  (bind _ashud_inimigo (cast `/Game/Caracter/HUDS/HUD_Inimigo` (`WidgetComponent.GetUserWidgetObject` (`self.Widget`))))
  (`ProgressBar.SetPercent` (`/Game/Caracter/HUDS/HUD_Inimigo.VidaDoInimigo` _ashud_inimigo) (`self.HealthInim`)))

(event `self.PawnSensing.OnSeePawn`
  (params (Pawn :type "Pawn Object Reference"))
  ;[1 1 1] Seguir jogador
  (`|AIMoveTo` self (0.0 0.0 0.0) Pawn))

(event `self.Box.OnComponentBeginOverlap`
  (params (OverlappedComponent :type "PrimitiveComponent Object Reference") (OtherActor :type "Actor Object Reference") (OtherComp :type "PrimitiveComponent Object Reference") (OtherBodyIndex :type Integer) (bFromSweep :type Boolean) (SweepResult :type "HitResult Structure (by ref)"))
  ;[1 1 1] Animação soco
  (bind _asbp_third_person_character (cast `/Game/Caracter/Blueprints/BP_ThirdPersonCharacter` OtherActor))
  (bind _output_get (set `self.Player` _asbp_third_person_character))
  (`/Engine/EditorBlueprintResources/StandardMacros.DoOnce` false :!label _label
    (:`Completed`
      (`AnimInstance.Montage_Play` (`SkeletalMeshComponent.GetAnimInstance` (`self.Mesh`)) "/Game/Caracter/Animacoes/AnimacaoInimigo/Anim/Sword_And_Shield_Slash_Anim_mixamo_com_Montage.Sword_And_Shield_Slash_Anim_mixamo_com_Montage" 1.0 "MontageLength" 0.0 true)
      (`GameplayStatics.ApplyDamage` _output_get 0.05))))

(event `resetF`
  ;[1 1 1] Animação soco
  (goto _label :!via `Reset`))

(event `self.Box.OnComponentEndOverlap`
  (params (OverlappedComponent :type "PrimitiveComponent Object Reference") (OtherActor :type "Actor Object Reference") (OtherComp :type "PrimitiveComponent Object Reference") (OtherBodyIndex :type Integer))
  ;[1 1 1] Animação soco
  (cast `/Game/Caracter/Blueprints/BP_ThirdPersonCharacter` OtherActor)
  (`KismetSystemLibrary.Delay` 1.0)
  (`self.resetF`))

(fn `UserConstructionScript`)