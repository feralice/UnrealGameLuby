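; BP_Porta is a door in Zona3 that swings open when any actor overlaps it.
; ActorBeginOverlap calls the AbrirPorta event, which plays Timeline_0 from the start to drive the Porta component's relative yaw.
; There is no actor filter or closing logic, so each overlap replays the swing.
; An unconnected leftover attempt to open only after BP_InimArma and BP_InimCorpo enemies die never runs, noted as not working.
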(event `AbrirPorta`
  (bind (_direction _abrirporta) (`Timeline|Timeline_0` :!via `PlayFromStart`)
    (:`Update`
      (`SceneComponent.K2_SetRelativeRotation` (`self.porta`) (`KismetMathLibrary.MakeRotator` 0.0 0.0 _abrirporta) false false))))

(event `self.ReceiveActorBeginOverlap`
  (params (OtherActor :type "Actor Object Reference"))
  ;[1 1 1] Chama a função abrir porta
  (`self.AbrirPorta`))

(fn `UserConstructionScript`)