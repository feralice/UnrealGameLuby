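; Zone 2 Simon-style memory puzzle: players repeat a random sequence of colored lights and notes to open a door.
; Pressing Use inside the trigger builds the difficulty-based playlist, plays it recursively with delays, then starts listening.
; CheckNote compares inputs and counts hits, PlayNotes handles light/sound or failure damage, and colored triggers set platform flags for external use.
; The door timeline plays on BoxPorta overlap once hits equal sequence length.
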(event `InputAction|Use`
  (params (Key :type "Key Structure"))
  ;[1 1 1] Player trtigger overlap eventos
  (:`Pressed`
    (if (not (or (`self.isListening`) (`self.isPlaying`)))
      (`/Engine/EditorBlueprintResources/StandardMacros.Gate` true :!label _label
        (:`Exit`
          (`self.setUpDificuldade`)
          (`self.CriaPlaylist`))))))

(event `self.trigger.OnComponentBeginOverlap`
  (params (OverlappedComponent :type "PrimitiveComponent Object Reference") (OtherActor :type "Actor Object Reference") (OtherComp :type "PrimitiveComponent Object Reference") (OtherBodyIndex :type Integer) (bFromSweep :type Boolean) (SweepResult :type "HitResult Structure (by ref)"))
  ;[1 1 1] Player trtigger overlap eventos
  (bind _asbp_third_person_character (cast `/Game/Caracter/Blueprints/BP_ThirdPersonCharacter` OtherActor))
  (set `self.player` _asbp_third_person_character)
  (`self.EnableInput` (`GameplayStatics.GetPlayerController` 0))
  (goto _label :!via `Open`))

(event `self.trigger.OnComponentEndOverlap`
  (params (OverlappedComponent :type "PrimitiveComponent Object Reference") (OtherActor :type "Actor Object Reference") (OtherComp :type "PrimitiveComponent Object Reference") (OtherBodyIndex :type Integer))
  ;[1 1 1] Player trtigger overlap eventos
  (cast `/Game/Caracter/Blueprints/BP_ThirdPersonCharacter` OtherActor)
  (`self.DisableInput` (`GameplayStatics.GetPlayerController` 0))
  (goto _label :!via `Close`))

(event `setUpDificuldade`
  ;[1 1 1] Seta a dificuldade
  (`KismetArrayLibrary.Array_Clear` (`self.Playlist`))
  (switch `int` (`self.dificuldade`)
    (:`1`
      (set `self.NotasParaLembrar` 7)
      (set `self.Speed` 1.5))))

(event `CriaPlaylist`
  ;[1 1 1] Adicionando notas para a playlist
  (while (< (`KismetArrayLibrary.Array_Length` (`self.Playlist`)) (`self.NotasParaLembrar`))
    (`KismetArrayLibrary.Array_Add` (`self.Playlist`) (`KismetMathLibrary.RandomIntegerInRange` 0 3)))
  (`self.PlayPlaylist`))

(event `PlayPlaylist`
  ;[1 1 1] Toca notas
  (if (not (`self.isListening`))
    (if (< (`self.notasTocadas`) (`self.NotasParaLembrar`))
      (set `self.isPlaying` true)
      (switch `int` (`|GetArrayItem` (`self.Playlist`) (`self.notasTocadas`))
        (:`0`
          (`self.PlayNotes` false (`self.Blue_light`) "/Game/Caracter/Materiais/MI_Azul_Acesso.MI_Azul_Acesso" "/Game/Caracter/Sons/zona2Sons/do.do" "/Game/Caracter/Materiais/MI_Azul.MI_Azul"))
        (:`1`
          (`self.PlayNotes` false (`self.Red_light`) "/Game/Caracter/Materiais/MI_Vermelho_Acesso.MI_Vermelho_Acesso" "/Game/Caracter/Sons/zona2Sons/re.re" "/Game/Caracter/Materiais/MI_Vermelho.MI_Vermelho"))
        (:`2`
          (`self.PlayNotes` false (`self.Yellow_light`) "/Game/Caracter/Materiais/MI_Amarelo_Acesso.MI_Amarelo_Acesso" "/Game/Caracter/Sons/zona2Sons/mi.mi" "/Game/Caracter/Materiais/MI_Amarelo.MI_Amarelo"))
        (:`3`
          (`self.PlayNotes` false (`self.Green_light`) "/Game/Caracter/Materiais/MI_Verde_Acesso.MI_Verde_Acesso" "/Game/Caracter/Sons/zona2Sons/fa.fa" "/Game/Caracter/Materiais/MI_Verde.MI_Verde")))
      (set `self.notasTocadas` (+ (`self.notasTocadas`) 1))
      (if (< (`self.notasTocadas`) (`self.NotasParaLembrar`))
        (`KismetSystemLibrary.Delay` (`self.Speed`))
        (`self.PlayPlaylist`)
        (else
          (set `self.isPlaying` false)
          (set `self.isListening` true)))
      (else
        (set `self.isListening` true)))))

(event `PlayNotes`
  (params (isFail :type Boolean) (light :type "StaticMeshComponent Object Reference") (onMaterial :type "MaterialInterface Object Reference") (Sound :type "SoundBase Object Reference") (offMaterial :type "MaterialInterface Object Reference"))
  (bind _returnvalue (`SceneComponent.K2_GetComponentLocation` light))
  ;[1 1 1] Toca as notas
  (if isFail
    (`GameplayStatics.PlaySoundAtLocation` "/Game/StarterContent/Audio/Explosion01.Explosion01" _returnvalue (struct) (`self.Volume Multiplier`) 1.0 0.0 null null null null)
    (`GameplayStatics.ApplyDamage` (`self.player`) 0.2)
    (else
      (`PrimitiveComponent.SetMaterial` light 0 onMaterial)
      (`GameplayStatics.PlaySoundAtLocation` Sound _returnvalue (struct) (`self.Volume Multiplier`) 1.0 0.0 null null null null)
      (`KismetSystemLibrary.Delay` 0.5)
      (`PrimitiveComponent.SetMaterial` light 0 offMaterial))))

(event `self.Red_trigger.OnComponentBeginOverlap`
  (params (OverlappedComponent :type "PrimitiveComponent Object Reference") (OtherActor :type "Actor Object Reference") (OtherComp :type "PrimitiveComponent Object Reference") (OtherBodyIndex :type Integer) (bFromSweep :type Boolean) (SweepResult :type "HitResult Structure (by ref)"))
  ;[1 1 1] Verificar se jogador está na plataforma para atirar em cada butão respectivo de sua cor da plataforma
  (set `self.estaNoVermelho` true))

(event `self.Red_trigger.OnComponentEndOverlap`
  (params (OverlappedComponent :type "PrimitiveComponent Object Reference") (OtherActor :type "Actor Object Reference") (OtherComp :type "PrimitiveComponent Object Reference") (OtherBodyIndex :type Integer))
  ;[1 1 1] Verificar se jogador está na plataforma para atirar em cada butão respectivo de sua cor da plataforma
  (set `self.estaNoVermelho` false))

(event `self.BoxPorta.OnComponentBeginOverlap`
  (params (OverlappedComponent :type "PrimitiveComponent Object Reference") (OtherActor :type "Actor Object Reference") (OtherComp :type "PrimitiveComponent Object Reference") (OtherBodyIndex :type Integer) (bFromSweep :type Boolean) (SweepResult :type "HitResult Structure (by ref)"))
  ;[1 1 1] Abrir porta quando jogador tiverr acertado todas as notas
  (cast `/Game/Caracter/Blueprints/BP_ThirdPersonCharacter` OtherActor)
  (if (== (`self.NotasParaLembrar`) (`self.numAcertos`))
    (bind (_direction _newtrack_2) (`Timeline|abrirPorta` :!via `PlayFromStart`)
      (:`Update`
        (`SceneComponent.K2_SetRelativeRotation` (`self.Porta`) (`KismetMathLibrary.MakeRotator` 0.0 0.0 _newtrack_2) false false)))))

(event `self.Blue_trigger.OnComponentBeginOverlap`
  (params (OverlappedComponent :type "PrimitiveComponent Object Reference") (OtherActor :type "Actor Object Reference") (OtherComp :type "PrimitiveComponent Object Reference") (OtherBodyIndex :type Integer) (bFromSweep :type Boolean) (SweepResult :type "HitResult Structure (by ref)"))
  ;[1 1 1] Verificar se jogador está na plataforma para atirar em cada butão respectivo de sua cor da plataforma
  (set `self.estaNoAzul` true))

(event `self.Blue_trigger.OnComponentEndOverlap`
  (params (OverlappedComponent :type "PrimitiveComponent Object Reference") (OtherActor :type "Actor Object Reference") (OtherComp :type "PrimitiveComponent Object Reference") (OtherBodyIndex :type Integer))
  ;[1 1 1] Verificar se jogador está na plataforma para atirar em cada butão respectivo de sua cor da plataforma
  (set `self.estaNoAzul` false))

(event `self.Green_trigger.OnComponentBeginOverlap`
  (params (OverlappedComponent :type "PrimitiveComponent Object Reference") (OtherActor :type "Actor Object Reference") (OtherComp :type "PrimitiveComponent Object Reference") (OtherBodyIndex :type Integer) (bFromSweep :type Boolean) (SweepResult :type "HitResult Structure (by ref)"))
  ;[1 1 1] Verificar se jogador está na plataforma para atirar em cada butão respectivo de sua cor da plataforma
  (set `self.estaNoVerde` true))

(event `self.Green_trigger.OnComponentEndOverlap`
  (params (OverlappedComponent :type "PrimitiveComponent Object Reference") (OtherActor :type "Actor Object Reference") (OtherComp :type "PrimitiveComponent Object Reference") (OtherBodyIndex :type Integer))
  ;[1 1 1] Verificar se jogador está na plataforma para atirar em cada butão respectivo de sua cor da plataforma
  (set `self.estaNoVerde` false))

(event `self.yellow_trigger.OnComponentBeginOverlap`
  (params (OverlappedComponent :type "PrimitiveComponent Object Reference") (OtherActor :type "Actor Object Reference") (OtherComp :type "PrimitiveComponent Object Reference") (OtherBodyIndex :type Integer) (bFromSweep :type Boolean) (SweepResult :type "HitResult Structure (by ref)"))
  ;[1 1 1] Verificar se jogador está na plataforma para atirar em cada butão respectivo de sua cor da plataforma
  (set `self.estaNoAmarelo` true))

(event `self.yellow_trigger.OnComponentEndOverlap`
  (params (OverlappedComponent :type "PrimitiveComponent Object Reference") (OtherActor :type "Actor Object Reference") (OtherComp :type "PrimitiveComponent Object Reference") (OtherBodyIndex :type Integer))
  ;[1 1 1] Verificar se jogador está na plataforma para atirar em cada butão respectivo de sua cor da plataforma
  (set `self.estaNoAmarelo` false))

(fn `CheckNote`
  (params (NoteToCheck :type Integer))
  (returns (isFail :type Boolean))
  (bind _playerplaylist (`self.PlayerPlaylist`))
  (bind _returnvalue (== (`local.NoteToCheck`) (`|GetArrayItem` (`self.Playlist`) (- (`KismetArrayLibrary.Array_Length` _playerplaylist) 1))))
  ;[1 1 1] Coloca as escolhas do jogador e compara
  (`KismetArrayLibrary.Array_Add` _playerplaylist NoteToCheck)
  (`|ExecutionSequence`
    (:`then_0`
      (if _returnvalue
        (set `self.numAcertos` (+ (`self.numAcertos`) 1))))
    (:`then_1`
      (return (not _returnvalue)))))

(fn `UserConstructionScript`)